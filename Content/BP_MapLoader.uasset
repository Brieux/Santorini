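; Map loader that builds the grid of BP_Cell actors on BeginPlay, then lets the player's BP_Pawn place workers and centers it over the map.
; Nested loops with inclusive bounds spawn and store cells in a flat array.
; AddNeighboor links each cell to its orthogonal and diagonal neighbours through index arithmetic.
; That arithmetic uses SizeMapX + 1 as stride, while Y is the inner loop, so it assumes a square map.
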(event `self.ReceiveBeginPlay`
  (set `self.Count` 0)
  (for _index (range (+ (`self.SizeMapX`) 1))
    (for _index_2 (range (+ (`self.SizeMapY`) 1))
      (bind _returnvalue (`|SpawnActorFromClass` "/Game/BP_Cell.BP_Cell_C" (`KismetMathLibrary.MakeTransform` (`KismetMathLibrary.MakeVector` (* _index (`self.SizeCellX`)) (* _index_2 (`self.SizeCellY`)))) "Undefined" "MultiplyWithRoot" null null))
      (set `self.Count` (+ (`self.Count`) 1))
      (`KismetArrayLibrary.Array_AddUnique` (`self.Cells`) _returnvalue)))
  (`self.AddNeighboor`)
  (bind _asbp_pawn (cast `/Game/BP_Pawn` (`GameplayStatics.GetPlayerPawn` 0)))
  (set `/Game/BP_Pawn.isAllowToPlaceWorkers` true _asbp_pawn)
  (`self.PlaceCamera`))

(event `PlaceCamera`
  (`self.K2_SetActorLocation` (`GameplayStatics.GetPlayerPawn` 0) (`KismetMathLibrary.MakeVector` (+ (* (/ (`self.SizeMapX`) 2) (`self.SizeCellX`)) (/ (`self.SizeCellX`) 2.0)) (+ (* (/ (`self.SizeMapY`) 2) (`self.SizeCellY`)) (/ (`self.SizeCellY`) 2.0))) false false))

(event `AddNeighboor`
  (for (_array_element _array_index) (`self.Cells`)
    (`|ExecutionSequence`
      (:`then_0`
        ;[1 1 1] Classique
        (`|ExecutionSequence`
          (:`then_0`
            (if (not (== (mod (+ _array_index 1) (+ (`self.SizeMapX`) 1)) 0))
              (bind _output (`|GetArrayItem` (`self.Cells`) (+ _array_index 1)))
              (`/Engine/EditorBlueprintResources/StandardMacros.IsValid` _output
                (:`Is Valid`
                  (`KismetArrayLibrary.Array_Add` (`/Game/BP_Cell.NeighboorCells` _array_element) _output)))))
          (:`then_1`
            (if (not (== (mod _array_index (+ (`self.SizeMapX`) 1)) 0))
              (bind _output_2 (`|GetArrayItem` (`self.Cells`) (- _array_index 1)))
              (`/Engine/EditorBlueprintResources/StandardMacros.IsValid` _output_2
                (:`Is Valid`
                  (`KismetArrayLibrary.Array_Add` (`/Game/BP_Cell.NeighboorCells` _array_element) _output_2)))))
          (:`then_2`
            (bind _output_3 (`|GetArrayItem` (`self.Cells`) (+ _array_index (+ (`self.SizeMapX`) 1))))
            (`/Engine/EditorBlueprintResources/StandardMacros.IsValid` _output_3
              (:`Is Valid`
                (`KismetArrayLibrary.Array_Add` (`/Game/BP_Cell.NeighboorCells` _array_element) _output_3))))
          (:`then_3`
            (bind _output_4 (`|GetArrayItem` (`self.Cells`) (- _array_index (+ (`self.SizeMapX`) 1))))
            (`/Engine/EditorBlueprintResources/StandardMacros.IsValid` _output_4
              (:`Is Valid`
                (`KismetArrayLibrary.Array_Add` (`/Game/BP_Cell.NeighboorCells` _array_element) _output_4))))))
      (:`then_1`
        ;[1 1 1] Diagonale
        (`|ExecutionSequence`
          (:`then_0`
            (bind _returnvalue (+ _array_index 1))
            (if (not (== (mod _returnvalue (+ (`self.SizeMapX`) 1)) 0))
              (bind _output_5 (`|GetArrayItem` (`self.Cells`) (+ _returnvalue (+ (`self.SizeMapX`) 1))))
              (`/Engine/EditorBlueprintResources/StandardMacros.IsValid` _output_5
                (:`Is Valid`
                  (`KismetArrayLibrary.Array_Add` (`/Game/BP_Cell.NeighboorCells` _array_element) _output_5)))))
          (:`then_1`
            (if (not (== (mod _returnvalue (+ (`self.SizeMapX`) 1)) 0))
              (bind _output_6 (`|GetArrayItem` (`self.Cells`) (- _returnvalue (+ (`self.SizeMapX`) 1))))
              (`/Engine/EditorBlueprintResources/StandardMacros.IsValid` _output_6
                (:`Is Valid`
                  (`KismetArrayLibrary.Array_Add` (`/Game/BP_Cell.NeighboorCells` _array_element) _output_6)))))
          (:`then_2`
            (if (not (== (mod _array_index (+ (`self.SizeMapX`) 1)) 0))
              (`|ExecutionSequence`
                (:`then_0`
                  (bind _returnvalue_2 (- _array_index 1))
                  (bind _output_7 (`|GetArrayItem` (`self.Cells`) (+ _returnvalue_2 (+ (`self.SizeMapX`) 1))))
                  (`/Engine/EditorBlueprintResources/StandardMacros.IsValid` _output_7
                    (:`Is Valid`
                      (`KismetArrayLibrary.Array_Add` (`/Game/BP_Cell.NeighboorCells` _array_element) _output_7))))
                (:`then_1`
                  (bind _output_8 (`|GetArrayItem` (`self.Cells`) (- _returnvalue_2 (+ (`self.SizeMapX`) 1))))
                  (`/Engine/EditorBlueprintResources/StandardMacros.IsValid` _output_8
                    (:`Is Valid`
                      (`KismetArrayLibrary.Array_Add` (`/Game/BP_Cell.NeighboorCells` _array_element) _output_8))))))))))))

(fn `UserConstructionScript`)