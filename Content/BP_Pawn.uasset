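; Player pawn running a two-player, turn-based god-pick, move-and-build board game, with an orbit/zoom camera and selection UI.
; Tick traces under the cursor to select cells or workers, restricting picks to valid neighbours during an action.
; Clicks advance a boolean-driven flow: place four workers alternately, then select, move and build each turn.
; Reaching level three wins, as does leaving the opponent without options, then the map reloads.
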(event `self.ReceiveTick`
  (params (DeltaSeconds :type "Float (single-precision)"))
  (bind _cellselected (`self.CellSelected`))
  (bind _cellselected_2 (`self.CellSelected`))
  (bind _cellselected_3 (`self.CellSelected`))
  (bind _workerselected (`self.WorkerSelected`))
  (bind _workerselected_2 (`self.WorkerSelected`))
  (bind _hitresult (`PlayerController.GetHitResultUnderCursorForObjects` (`GameplayStatics.GetPlayerController` 0) (`|MakeArray` "ObjectTypeQuery2" :!type "EObjectTypeQuery Enum") true))
  (bind _hitresult_2 (`PlayerController.GetHitResultUnderCursorForObjects` (`GameplayStatics.GetPlayerController` 0) (`|MakeArray` "ObjectTypeQuery2" :!type "EObjectTypeQuery Enum") true))
  ;[1 1 1] HighlightCellOrWorker
  (if (`self.Play?`)
    (if (`|GetInputActionValue`)
      _
      (elif (`self.BlockSelection`)
        (if (or (`self.LookingForMovement`) (`self.NeedConstruction`))
          (if (`GameplayStatics.BreakHitResult` _hitresult)
            (bind _asbp_cell (cast `/Game/BP_Cell` (`.HitActor` (`GameplayStatics.BreakHitResult` _hitresult)))
              (:`then`
                (if (`/Game/BP_Cell.isValidNeighboor` _asbp_cell)
                  (set `self.CellSelected` _asbp_cell)))
              (:`CastFailed`
                (set `self.CellSelected` null)))
            (else
              (set `self.CellSelected` null))))
        (elif (`GameplayStatics.BreakHitResult` _hitresult_2)
          ;;[1 1 1] CellSelection
          (bind _asbp_cell_2 (cast `/Game/BP_Cell` (`.HitActor` (`GameplayStatics.BreakHitResult` _hitresult_2)))
            (:`then`
              (if (!= _asbp_cell_2 (`self.CellSelected`))
                (`/Engine/EditorBlueprintResources/StandardMacros.IsValid` _cellselected
                  (:`Is Valid`
                    (set `/Game/BP_Cell.isSelected` false _cellselected)
                    (`/Game/BP_Cell.IsSelectedToggle` _cellselected))
                  (:`Is Not Valid`
                    _))
                (bind _output_get (set `self.CellSelected` _asbp_cell_2))
                (set `/Game/BP_Cell.isSelected` true _output_get)
                (`/Game/BP_Cell.IsSelectedToggle` _output_get)
                (`/Engine/EditorBlueprintResources/StandardMacros.IsValid` _workerselected :!label _label
                  (:`Is Valid`
                    (set `/Game/BP_Ouvrier.is Selected` false _workerselected)
                    (`/Game/BP_Ouvrier.SwitchColor` _workerselected)
                    (set `self.WorkerSelected` null)))))
            (:`CastFailed`
              ;;[1 1 1] WorkerSelection
              (bind _asbp_ouvrier (cast `/Game/BP_Ouvrier` (`.HitActor` (`GameplayStatics.BreakHitResult` _hitresult_2))))
              (`/Engine/EditorBlueprintResources/StandardMacros.IsValid` _cellselected_2
                (:`Is Valid`
                  (set `/Game/BP_Cell.isSelected` false _cellselected_2)
                  (`/Game/BP_Cell.IsSelectedToggle` _cellselected_2)
                  (set `self.CellSelected` null))
                (:`Is Not Valid`
                  _))
              (if (!= _asbp_ouvrier (`self.WorkerSelected`))
                (`/Engine/EditorBlueprintResources/StandardMacros.IsValid` _workerselected_2
                  (:`Is Valid`
                    (set `/Game/BP_Ouvrier.is Selected` false _workerselected_2)
                    (`/Game/BP_Ouvrier.SwitchColor` _workerselected_2))
                  (:`Is Not Valid`
                    _))
                (bind _output_get_2 (set `self.WorkerSelected` _asbp_ouvrier))
                (if (== (`/Game/BP_Ouvrier.isJ1` _output_get_2) (`self.Player1`))
                  (set `/Game/BP_Ouvrier.is Selected` true _workerselected_2)
                  (`/Game/BP_Ouvrier.SwitchColor` _workerselected_2)))))
          (else
            (`/Engine/EditorBlueprintResources/StandardMacros.IsValid` _cellselected_3
              (:`Is Valid`
                (set `/Game/BP_Cell.isSelected` false _cellselected_3)
                (`/Game/BP_Cell.IsSelectedToggle` _cellselected_3)
                (set `self.CellSelected` null)
                (goto _label))
              (:`Is Not Valid`
                (goto _label)))))))))

(event `self.ReceivePossessed`
  (params (NewController :type "Controller Object Reference"))
  ;[1 1 1] Init
  (bind _asplayer_controller (cast `PlayerController` NewController))
  (message `EnhancedInputSubsystemInterface.AddMappingContext` (pcsubsystem `EnhancedInputLocalPlayerSubsystem` _asplayer_controller) "/Game/Input/IMC_Input.IMC_Input" 0 (struct)))

(event `DefineGod`
  (params (GodSelected :type "/Game/Enum_God Enum" :default "NewEnumerator0"))
  ;[1 1 1] Init
  ;;[1 1 1] ChooseGodInit
  (`/Engine/EditorBlueprintResources/StandardMacros.Gate` false :!label _label_2
    (:`Exit`
      (`/Engine/EditorBlueprintResources/StandardMacros.FlipFlop`
        (:`A`
          (set `self.J1God` GodSelected))
        (:`B`
          (set `self.J2God` GodSelected)
          (`self.BeginGame`)
          (goto _label_2 :!via `Close`))))))

(event `self.ReceiveBeginPlay`
  ;[1 1 1] Init
  (set `PlayerController.bShowMouseCursor` true (`GameplayStatics.GetPlayerController` 0))
  (bind _returnvalue (`|CreateWidget` "/Game/WBP_InterfaceSelection.WBP_InterfaceSelection_C"))
  (bind _output_get (set `self.GodUI` _returnvalue))
  (`UserWidget.AddToViewport` _output_get 0)
  (set `self.GameplayStatement` "NewEnumerator4"))

(event `BeginGame`
  ;[1 1 1] Init
  (`Widget.RemoveFromParent` (`self.GodUI`))
  (bind _returnvalue (`|CreateWidget` "/Game/WBP_InGameSelection.WBP_InGameSelection_C"))
  (bind _output_get (set `self.Interface` _returnvalue))
  (`UserWidget.AddToViewport` _output_get 0)
  (set `self.Play?` true)
  (set `self.GameplayStatement` "NewEnumerator0"))

(event `EnhancedInput|/Game/Input/IA_Move`
  (params (ActionValue :type "Float (double-precision)") (ElapsedSeconds :type "Float (double-precision)") (TriggeredSeconds :type "Float (double-precision)") (InputAction :type "InputAction Object Reference" :default "/Game/Input/IA_Move.IA_Move"))
  ;[1 1 1] CameraMovement
  (:`Triggered`
    (`SceneComponent.K2_AddWorldRotation` (`self.SpringArm`) (`KismetMathLibrary.MakeRotator` 0.0 0.0 ActionValue) false false)))

(event `EnhancedInput|/Game/Input/IA_ConfirmTurn`
  (params (ActionValue :type Boolean) (ElapsedSeconds :type "Float (double-precision)") (TriggeredSeconds :type "Float (double-precision)") (InputAction :type "InputAction Object Reference" :default "/Game/Input/IA_ConfirmTurn.IA_ConfirmTurn"))
  (bind _returnvalue (`GameplayStatics.GetPlayerController` 0))
  (bind (_locationx _locationy) (`PlayerController.GetMousePosition` _returnvalue))
  ;[1 1 1] CameraMovement
  (:`Triggered`
    (set `PlayerController.bShowMouseCursor` (not ActionValue) _returnvalue :!label _label_3))
  (:`Started`
    (set `self.Location X` _locationx)
    (set `self.Location Y` _locationy))
  (:`Completed`
    (`PlayerController.SetMouseLocation` _returnvalue (`KismetMathLibrary.FTrunc` (`self.Location X`)) (`KismetMathLibrary.FTrunc` (`self.Location Y`)))
    (goto _label_3)))

(event `EnhancedInput|/Game/Input/IA_ConfirmClick`
  (params (ActionValue :type Boolean) (ElapsedSeconds :type "Float (double-precision)") (TriggeredSeconds :type "Float (double-precision)") (InputAction :type "InputAction Object Reference" :default "/Game/Input/IA_ConfirmClick.IA_ConfirmClick"))
  (:`Completed`
    (if (`self.isAllowToPlaceWorkers`)
      (`self.AddWorkerOnCell`)
      (elif (not (`self.BlockSelection`))
        (`self.SelectValidWorker`)
        (elif (not (`self.NeedConstruction`))
          (`self.MoveWorkerOnCell`)
          (else
            (`self.Construct`)))))))

(event `EnhancedInput|/Game/Input/IA_Zoom`
  (params (ActionValue :type "Float (double-precision)") (ElapsedSeconds :type "Float (double-precision)") (TriggeredSeconds :type "Float (double-precision)") (InputAction :type "InputAction Object Reference" :default "/Game/Input/IA_Zoom.IA_Zoom"))
  (bind _springarm (`self.SpringArm`))
  ;[1 1 1] CameraMovement
  (:`Triggered`
    (set `SpringArmComponent.TargetArmLength` (+ (`SpringArmComponent.TargetArmLength` _springarm) (* (* ActionValue -1.0) 5.0)) _springarm)))

(event `EnhancedInput|/Game/Input/IA_Turn`
  (params (ActionValue :type "Float (double-precision)") (ElapsedSeconds :type "Float (double-precision)") (TriggeredSeconds :type "Float (double-precision)") (InputAction :type "InputAction Object Reference" :default "/Game/Input/IA_Turn.IA_Turn"))
  (bind _springarm (`self.SpringArm`))
  (bind (_relativerotation_roll _relativerotation_pitch _relativerotation_yaw) (`KismetMathLibrary.BreakRotator` (`SceneComponent.RelativeRotation` _springarm)))
  ;[1 1 1] CameraMovement
  (:`Triggered`
    (if (`|GetInputActionValue`)
      (`SceneComponent.K2_AddLocalRotation` _springarm (`KismetMathLibrary.MakeRotator` 0.0 ActionValue) false false)
      (`SceneComponent.K2_SetRelativeRotation` _springarm (`KismetMathLibrary.MakeRotator` _relativerotation_roll (`KismetMathLibrary.FClamp` _relativerotation_pitch -70.0 -20.0) _relativerotation_yaw) false false))))

(event `EnhancedInput|/Game/Input/IA_CancelSelection`
  (params (ActionValue :type Boolean) (ElapsedSeconds :type "Float (double-precision)") (TriggeredSeconds :type "Float (double-precision)") (InputAction :type "InputAction Object Reference" :default "/Game/Input/IA_CancelSelection.IA_CancelSelection"))
  (bind _workerselected (`self.WorkerSelected`))
  ;[1 1 1] CancelSelection
  (:`Started`
    (if (`self.BlockSelection`)
      (set `self.BlockSelection` false)
      (set `/Game/BP_Ouvrier.isBlockedInSelection` false _workerselected)
      (`/Game/BP_Ouvrier.SwitchColor` _workerselected)
      (`/Game/BP_Cell.UncallNeighboor` (`/Game/BP_Ouvrier.CurrentCell` _workerselected))
      (set `self.LookingForMovement` false))))

(event `AddWorkerOnCell`
  (bind _cellselected (`self.CellSelected`))
  (bind _cellselected_2 (`self.CellSelected`))
  (bind (_returnvalue_x _returnvalue_y _returnvalue_z) (`KismetMathLibrary.BreakVector` (`self.K2_GetActorLocation` _cellselected)))
  ;[1 1 1] OnClickGameplay
  ;;[1 1 1] WorkersPlacementInInit
  (`/Engine/EditorBlueprintResources/StandardMacros.IsValid` _cellselected
    (:`Is Valid`
      (if (not (`/Game/BP_Cell.AlreadyWorker` _cellselected_2))
        (bind _returnvalue (`|SpawnActorFromClass` "/Game/BP_Ouvrier.BP_Ouvrier_C" (`KismetMathLibrary.MakeTransform` (`KismetMathLibrary.MakeVector` _returnvalue_x _returnvalue_y (+ _returnvalue_z 25.0))) "Undefined" "MultiplyWithRoot" null (`self.Player1`) (`self.CellSelected`) null))
        (set `/Game/BP_Cell.AlreadyWorker` true _cellselected_2)
        (`/Game/BP_Ouvrier.SwitchColor` _returnvalue)
        (bind _output_get (set `self.CountWorkers` (+ (`self.CountWorkers`) 1)))
        (set `self.Player1` (not (`self.Player1`)))
        (if (> _output_get 3)
          (set `self.isAllowToPlaceWorkers` false))))))

(event `DidPlayerLose`
  ;[1 1 1] EndOfGame
  ;;[1 1 1] LooseCondition
  (`KismetArrayLibrary.Array_Clear` (`self.CurrentWorker`))
  (bind _outactors (`GameplayStatics.GetAllActorsOfClass` "/Game/BP_Ouvrier.BP_Ouvrier_C"))
  (for _array_element _outactors
    (if (== (`self.Player1`) (`/Game/BP_Ouvrier.isJ1` _array_element))
      (`KismetArrayLibrary.Array_Add` (`self.CurrentWorker`) _array_element)))
  (set `self.hasLoose` true)
  (for _array_element_2 (`self.CurrentWorker`) :!label _label_4
    (bind _hasmoveavailable (`/Game/BP_Ouvrier.CalculateLoose` _array_element_2))
    (bind _output_get (set `self.hasLoose` (not _hasmoveavailable)))
    (if (not _output_get)
      (`self.breakLoop`)))
  (if (`self.hasLoose`)
    (set `self.Player1` (not (`self.Player1`)))
    (`self.Win`)))

(event `breakLoop`
  ;[1 1 1] EndOfGame
  ;;[1 1 1] LooseCondition
  (goto _label_4 :!via `Break`))

(event `SelectValidWorker`
  (bind _workerselected (`self.WorkerSelected`))
  (bind _workerselected_2 (`self.WorkerSelected`))
  ;[1 1 1] OnClickGameplay
  ;;[1 1 1] SelectWorkerToMove
  (`/Engine/EditorBlueprintResources/StandardMacros.IsValid` _workerselected
    (:`Is Valid`
      (if (== (`/Game/BP_Ouvrier.isJ1` _workerselected) (`self.Player1`))
        (set `self.BlockSelection` true)
        (set `/Game/BP_Ouvrier.isBlockedInSelection` true _workerselected)
        (`/Game/BP_Cell.CallNeighboor` (`/Game/BP_Ouvrier.CurrentCell` _workerselected_2) false (`/Game/BP_Ouvrier.Level` _workerselected_2))
        (set `self.LookingForMovement` true)))))

(event `Win`
  (bind _interface (`self.Interface`))
  ;[1 1 1] EndOfGame
  ;;[1 1 1] ShowWin
  (`|PlayAnimationTimeRange` _interface (`/Game/WBP_InGameSelection.ShowWin` _interface)
    (:`then`
      (set `/Game/WBP_InGameSelection.isWinByJ1` (`self.Player1`) _interface))
    (:`Finished`
      (`KismetSystemLibrary.Delay` 5.0)
      (`GameplayStatics.OpenLevelBySoftObjectPtr` "/Game/MainMap.MainMap"))))

(event `MoveWorkerOnCell`
  (bind _workerselected (`self.WorkerSelected`))
  (bind _cellselected (`self.CellSelected`))
  (bind _workerselected_2 (`self.WorkerSelected`))
  (bind _cellselected_2 (`self.CellSelected`))
  (bind (_returnvalue_x _returnvalue_y _returnvalue_z) (`KismetMathLibrary.BreakVector` (`self.K2_GetActorLocation` _cellselected)))
  (bind _currentcell (`/Game/BP_Ouvrier.CurrentCell` _workerselected))
  ;[1 1 1] OnClickGameplay
  ;;[1 1 1] MoveWorkerOnCell
  (`/Engine/EditorBlueprintResources/StandardMacros.IsValid` _cellselected_2
    (:`Is Valid`
      (if (`/Game/BP_Cell.isValidNeighboor` _cellselected_2)
        (`SceneComponent.K2_SetWorldLocation` (`/Game/BP_Ouvrier.DefaultSceneRoot` _workerselected) (`KismetMathLibrary.MakeVector` _returnvalue_x _returnvalue_y (+ (+ _returnvalue_z 25.0) (* (`/Game/BP_Cell.Level` _cellselected) 50.0))) false false)
        (`/Game/BP_Cell.UncallNeighboor` _currentcell)
        (set `/Game/BP_Cell.AlreadyWorker` false _currentcell)
        (bind _output_get (set `/Game/BP_Ouvrier.CurrentCell` _cellselected _workerselected))
        (set `/Game/BP_Cell.AlreadyWorker` true _output_get)
        (bind _output_get_2 (set `/Game/BP_Ouvrier.Level` (`/Game/BP_Cell.Level` _output_get) (`self.WorkerSelected`)))
        (if (== _output_get_2 3)
          (`self.Win`)
          (else
            (set `self.LookingForMovement` false)
            (set `/Game/BP_Ouvrier.isBlockedInSelection` false _workerselected_2)
            (set `/Game/BP_Ouvrier.is Selected` false _workerselected_2)
            (`/Game/BP_Ouvrier.SwitchColor` _workerselected_2)
            (set `self.NeedConstruction` true)
            (`/Game/BP_Cell.CallNeighboor` (`/Game/BP_Ouvrier.CurrentCell` _workerselected_2) true 0)))))))

(event `Construct`
  (bind _cellselected (`self.CellSelected`))
  ;[1 1 1] OnClickGameplay
  ;;[1 1 1] Construct
  (`/Engine/EditorBlueprintResources/StandardMacros.IsValid` _cellselected
    (:`Is Valid`
      (if (`/Game/BP_Cell.isValidNeighboor` _cellselected)
        (`/Game/BP_Cell.AddLevel` _cellselected)
        (`/Game/BP_Cell.UncallNeighboor` (`/Game/BP_Ouvrier.CurrentCell` (`self.WorkerSelected`)))
        (set `self.Player1` (not (`self.Player1`)))
        (set `self.NeedConstruction` false)
        (set `self.BlockSelection` false)
        (`self.DidPlayerLose`)))))

(fn `UserConstructionScript`)