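; Board cell for a worker move-and-build game, tracking its level, selection and neighbor validity.
; CallNeighboor flags and recolors valid neighbors: unoccupied and below level 4, plus at most one level up when moving; UncallNeighboor resets them.
; AddLevel stacks a static mesh at a height and material set by the new level.
; CountDeplacementAvailable is a stub returning zero.
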(event `IsSelectedToggle`
  (bind _plane (`self.Plane`))
  (if (`self.isSelected`)
    (`PrimitiveComponent.SetMaterial` _plane 0 "/Game/Mat/Green.Green")
    (else
      (`PrimitiveComponent.SetMaterial` _plane 0 "/Game/Mat/Red.Red"))))

(event `CallNeighboor`
  (params (isBuild :type Boolean) (LevelCurrent :type Integer))
  (for _array_element (`self.NeighboorCells`)
    (if isBuild
      (bind _level (`/Game/BP_Cell.Level` _array_element))
      (bind _returnvalue (< _level 4))
      (bind _returnvalue_2 (not (`/Game/BP_Cell.AlreadyWorker` _array_element)))
      (if (and _returnvalue _returnvalue_2)
        (`self.ActivateNeighboorColour` _array_element :!label _label))
      (elif (and _returnvalue_2 _returnvalue (<= (- _level 1) LevelCurrent))
        (goto _label)))))

(event `ActivateNeighboorColour`
  (`PrimitiveComponent.SetMaterial` (`self.Plane`) 0 "/Game/Mat/Neighboor.Neighboor")
  (set `self.isValidNeighboor` true))

(event `UncallNeighboor`
  (for _array_element (`self.NeighboorCells`)
    (`self.DeactivateNeighboorColour` _array_element)))

(event `DeactivateNeighboorColour`
  (`PrimitiveComponent.SetMaterial` (`self.Plane`) 0 "/Game/Mat/Red.Red")
  (set `self.isValidNeighboor` false))

(event `AddLevel`
  (bind _level (`self.Level`))
  (`/Engine/EditorBlueprintResources/StandardMacros.IncrementInt` _level
    (:`  `
      (bind _returnvalue (`AddComponent|NODE_AddStaticMeshComponent-0` :`RelativeTransform` (`KismetMathLibrary.MakeTransform` (`KismetMathLibrary.MakeVector` 0.0 0.0 (`KismetMathLibrary.Conv_IntToDouble` (+ 25 (* (- _level 1) 50)))) (struct) (0.5 0.5 0.5))))
      (`PrimitiveComponent.SetMaterial` _returnvalue 0 (select `int` (`self.Level`) :`0` null :`1` "/Game/Mat/Level1.Level1" :`2` "/Game/Mat/Level2.Level2" :`3` "/Game/Mat/Level3.Level3" :`4` "/Game/Mat/Level4.Level4" :!type "MaterialInterface Object Reference")))))

(fn `Count Deplacement Available`
  (returns (Count :type Integer))
  (return 0))

(fn `UserConstructionScript`)